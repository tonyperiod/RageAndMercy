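; Doorway actor that opens once the player has collected a set number of items.
; On BeginPlay it binds a check to the FirstPersonGameMode's collected-item event.
; When the collected count equals NumberToOpen, it plays a stone-moving sound at Pillar1, eases the Light component downward over OverTime, then destroys itself.
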(event Custom|CheckIfRaise
  (if (== (Variables|Default|GetNumberToOpen) (- (Variables|/Game/AAMyStuff/Blueprints/FirstPersonGameMode.FirstPersonGameMode_C|GetTotalCollectibles (stale EventBeginPlay _asfirst_person_game_mode)) (Variables|/Game/AAMyStuff/Blueprints/FirstPersonGameMode.FirstPersonGameMode_C|Getcollectibles%20left (stale EventBeginPlay _asfirst_person_game_mode))))
    (Audio|PlaySoundatLocation "/Game/AAMyStuff/Audio/SFX/stonemove.stonemove" (Transformation|GetWorldLocation (Variables|Default|GetPillar1)) "0, 0, 0" 1.0 1.0 0.0 0 0 0)
    (Components|MoveComponentTo (Variables|Default|GetLight) "0, 0,-1200.000000" "0, 0, 0" false true (Variables|Default|GetOver%20Time) false)
    (Actor|DestroyActor)))

(event EventBeginPlay
  (bind _asfirst_person_game_mode (Utilities|Casting|CastToFirstPersonGameMode (Game|GetGameMode)))
  (EventDispatchers|BindEventtoCollectedItem _asfirst_person_game_mode (delegate Custom|CheckIfRaise)))

(fn ConstructionScript)