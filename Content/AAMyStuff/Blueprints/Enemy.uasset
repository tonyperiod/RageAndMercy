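; Enemy AI character that shoots magazine-limited bursts of randomly spread bullets, flees from the player and can be killed by the player's attack.
; Player overlap with FearRadius sets a timed IsFeared Blackboard key, and RunAway writes a random reachable escape point away from the player.
; An attacking player's capsule hit sets IsDead, launches and ragdolls the enemy, and fully heals the player via negative damage.
; It re-caches the player reference on revival.
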(event OnComponentBeginOverlap(FearRadius)
  (params (OverlappedComponent :type Primitive%20Component%20Object%20Reference) (OtherActor :type Actor%20Object%20Reference) (OtherComp :type Primitive%20Component%20Object%20Reference) (OtherBodyIndex :type Integer) (bFromSweep :type Boolean) (SweepResult :type Hit%20Result%20Structure%20%28by%20ref%29))
  ;[1 1 1] PlayerClose
  (Utilities|Casting|CastToFirstPersonCharacter OtherActor)
  (AI|Components|Blackboard|SetValueasBool (AI|GetBlackboard 0) (Utilities|Name|MakeLiteralName "IsFeared") true)
  (Variables|Default|SetBP_IsFeared true)
  (Utilities|FlowControl|Delay (Variables|Default|GetFearDuration))
  (AI|Components|Blackboard|SetValueasBool (AI|GetBlackboard 0) (Utilities|Name|MakeLiteralName "IsFeared") false)
  (Variables|Default|SetBP_IsFeared false))

(event OnComponentHit(CapsuleComponent)
  (params (HitComponent :type Primitive%20Component%20Object%20Reference) (OtherActor :type Actor%20Object%20Reference) (OtherComp :type Primitive%20Component%20Object%20Reference) (NormalImpulse :type Vector :default "0, 0, 0") (Hit :type Hit%20Result%20Structure%20%28by%20ref%29))
  (bind _returnvalue (Transformation|GetActorLocation OtherActor))
  (bind _returnvalue_2 (Transformation|GetActorLocation))
  (bind _playerref (Variables|Default|GetPlayerRef))
  (bind _returnvalue_3 (* _returnvalue -1.0))
  (bind _returnvalue_4 (+ _returnvalue_2 _returnvalue_3))
  (bind (_x _y) (Math|Vector|BreakVector _returnvalue_4))
  ;[1 1 1] Death Ragdoll
  (bind _asfirst_person_character (Utilities|Casting|CastToFirstPersonCharacter OtherActor))
  (if (Variables|/Game/AAMyStuff/Blueprints/FirstPersonCharacter.FirstPersonCharacter_C|GetIsAttack _asfirst_person_character)
    (AI|Components|Blackboard|SetValueasBool (AI|GetBlackboard 0) (Utilities|Name|MakeLiteralName "IsDead") true)
    (Character|LaunchCharacter (* (Math|Vector|MakeVector _x _y (.Z (Math|Vector|BreakVector _returnvalue_2))) (Variables|Default|GetLaunchStre)) false false)
    (Physics|SetSimulatePhysics (Variables|Character|GetMesh) true)
    ;[1 1 1] HealPlayer
    (Class|BPIDamagable|TakeDamage(Message) _playerref (- (Variables|/Game/AAMyStuff/Blueprints/FirstPersonCharacter.FirstPersonCharacter_C|GetHPCurrent _playerref) (Variables|/Game/AAMyStuff/Blueprints/FirstPersonCharacter.FirstPersonCharacter_C|GetHPMax _playerref)))))

(event Custom|StartShoot
  ;[1 1 1] Shooting
  ;;[1 1 1] current shot
  (bind _output_get (Variables|Default|SetCurrentShot (+ (Variables|Default|GetCurrentShot) 1.0)))
  ;;[1 1 1] Reload?
  (if (>= _output_get (Variables|Default|GetMagSize))
    (Variables|Default|SetIsReload true)
    (Variables|Default|SetIsFiring false)
    (else
      (Variables|Default|SetIsFiring true)
      ;;[1 1 1] shoot
      (CallFunction|FireBullet)
      (Variables|Default|SetShootingLoop ""))))

(event Custom|StartReload
  ;[1 1 1] Reload
  (Utilities|Time|ClearandInvalidateTimerbyHandle (Variables|Default|GetShootingLoop))
  (Utilities|FlowControl|Delay (Variables|Default|GetReload))
  (Variables|Default|SetIsReload false)
  (Variables|Default|SetCurrentShot 0.0))

(event Custom|StopShooting
  ;[1 1 1] StopShooting
  (Variables|Default|SetIsFiring false)
  (Utilities|Time|ClearandInvalidateTimerbyHandle (Variables|Default|GetShootingLoop)))

(event Custom|RunAway
  ;[1 1 1] Run Away
  (Animation|Montage|MontagePlay (Components|SkeletalMesh|GetAnimInstance (Variables|Character|GetMesh)) "/Game/AAMyStuff/Mesh+Anim/Enemy/EnemyRun.EnemyRun" 1.0 "MontageLength" 0.0 true)
  (CallFunction|GetEscapeVector))

(event Custom|Turn%20Around
  ;[1 1 1] Turn Around to run
  (bind _returnvalue (Animation|Montage|MontagePlay (Components|SkeletalMesh|GetAnimInstance (Variables|Character|GetMesh)) "/Game/AAMyStuff/Mesh+Anim/Enemy/EnemyTurn.EnemyTurn" 1.0 "MontageLength" 0.0 true))
  (Utilities|FlowControl|Delay _returnvalue))

(event Custom|PlayerRevived
  ;[1 1 1] For Checkpoints
  ;;[1 1 1] Recast to player
  ;;[1 1 1] Player Reference
  (bind _asfirst_person_character (Utilities|Casting|CastToFirstPersonCharacter (Game|GetPlayerCharacter 0)))
  (Variables|Default|SetPlayerRef _asfirst_person_character))

(event EventBeginPlay
  (Utilities|FlowControl|Sequence
    (:then_0
      ;[1 1 1] GetAnim
      (bind _asanim_bp_enemy (Utilities|Casting|CastToAnimBP_Enemy (Components|SkeletalMesh|GetAnimInstance (Variables|Character|GetMesh))))
      (Variables|Default|SetStartShooting _asanim_bp_enemy))
    (:then_1
      ;[1 1 1] SetNotFeared
      (AI|Components|Blackboard|SetValueasBool (AI|GetBlackboard 0) (Utilities|Name|MakeLiteralName "IsFeared") false))
    (:then_2
      ;[1 1 1] For Checkpoints
      ;;[1 1 1] Recast to player
      (bind _asfirst_person_game_mode (Utilities|Casting|CastToFirstPersonGameMode (Game|GetGameMode)))
      (EventDispatchers|BindEventtoPlayerIsRevived _asfirst_person_game_mode (delegate Custom|PlayerRevived)))
    (:then_3
      ;;[1 1 1] Player Reference
      (bind _asfirst_person_character (Utilities|Casting|CastToFirstPersonCharacter (Game|GetPlayerCharacter 0)))
      (Variables|Default|SetPlayerRef _asfirst_person_character))))

(fn ConstructionScript)

(fn FireBullet
  (bind _barrelref (Variables|Default|GetBarrelRef))
  ;[1 1 1] animation
  (Animation|Montage|MontagePlay (Components|SkeletalMesh|GetAnimInstance (Variables|Character|GetMesh)) "/Game/AAMyStuff/Mesh+Anim/Enemy/EnemyFiring.EnemyFiring" 1.0 "MontageLength" 0.0 true)
  ;[1 1 1] spawBullets
  (for _index (range 1 (Variables|Default|GetBulletNumber))
    (Game|SpawnActorfromClass "/Game/AAMyStuff/Blueprints/Bullets.Bullets_C" (Math|Transform|MakeTransform (Transformation|GetWorldLocation _barrelref) (CallFunction|GetSprayAngle (Variables|Default|GetMaxAngle) (Math|Vector|GetForwardVector _barrelref)) "0.100000,0.100000,0.100000") "AlwaysSpawn" 0 0)))

(fn GetSprayAngle
  (params (MaxAngle :type Float%20%28single-precision%29) (BarrelForward :type Vector))
  (return (Math|Rotator|MakeRotfromX (Math|Random|RandomUnitVectorinConeinDegrees BarrelForward MaxAngle))))

(fn GetEscapeVector
  (bind _returnvalue (Transformation|GetActorLocation))
  (bind _playerref (Variables|Default|GetPlayerRef))
  (bind _returnvalue_2 (Transformation|GetActorLocation _playerref))
  (bind _returnvalue_3 (Math|Rotator|FindLookatRotation _returnvalue _returnvalue_2))
  (bind _returnvalue_4 (Math|Vector|GetForwardVector _returnvalue_3))
  (bind _returnvalue_5 (* _returnvalue_4 -5e+02))
  (bind _returnvalue_6 (+ _returnvalue _returnvalue_5))
  (bind (_x _y) (Math|Vector|BreakVector _returnvalue_6))
  (AI|Components|Blackboard|SetValueasVector (AI|GetBlackboard 0) (Utilities|Name|MakeLiteralName "RunAwayLocation") (.RandomLocation (AI|Navigation|GetRandomReachablePointinRadius (Math|Vector|MakeVector _x _y (.Z (Math|Vector|BreakVector _returnvalue))) 1e+03 0 0))))