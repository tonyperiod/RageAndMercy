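; Enemy AI controller that runs the Enemy_BT behavior tree and feeds it player sightings from AI Perception.
; On begin play it starts the tree and sets the Can'tSeePlayer blackboard key to true.
; Perception updates for the FirstPersonCharacter write the sensed state to CanSeePlayer.
; A successful sense while IsRelax is set clears both Can'tSeePlayer and IsRelax, with nothing here restoring them afterwards.
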(event OnTargetPerceptionUpdated(AIPerception)
  (params (Actor :type Actor%20Object%20Reference) (Stimulus :type AI%20Stimulus%20Structure))
  (bind _returnvalue (AI|GetBlackboard 0))
  ;[1 1 1] ai perception
  (Utilities|Casting|CastToFirstPersonCharacter Actor)
  (AI|Components|Blackboard|SetValueasBool _returnvalue (Utilities|Name|MakeLiteralName "CanSeePlayer") (.bsuccessfullysensed Stimulus))
  (if (.bsuccessfullysensed Stimulus)
    (if (Variables|Default|GetIsRelax)
      (AI|Components|Blackboard|SetValueasBool _returnvalue (Utilities|Name|MakeLiteralName "Can'tSeePlayer") false)
      (Variables|Default|SetIsRelax false))))

(event EventBeginPlay
  (AI|RunBehaviorTree "/Game/AAMyStuff/Blueprints/Enemy_BT.Enemy_BT")
  (AI|Components|Blackboard|SetValueasBool (AI|GetBlackboard 0) (Utilities|Name|MakeLiteralName "Can'tSeePlayer") true))

(fn ConstructionScript)